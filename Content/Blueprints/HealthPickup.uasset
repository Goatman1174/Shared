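; HealthPickup is a spinning pickup actor that restores a fixed amount of health to a Gliding_Character.
; Tick uses a short Delay to throttle a steady yaw increment on the Scene component.
; Box overlap by a character below max health nudges Scene by a unit direction vector toward the first-person camera and adds clamped health.
; The actor destroys itself after a brief delay, before that move finishes.
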(event `self.ReceiveTick`
  (params (DeltaSeconds :type "Float (single-precision)"))
  (bind (_returnvalue_roll _returnvalue_pitch _returnvalue_yaw) (`KismetMathLibrary.BreakRotator` (`SceneComponent.K2_GetComponentRotation` (`self.Scene`))))
  (`KismetSystemLibrary.Delay` 0.05)
  (`SceneComponent.K2_SetWorldRotation` (`self.Scene`) (`KismetMathLibrary.MakeRotator` _returnvalue_roll _returnvalue_pitch (+ _returnvalue_yaw 1.0)) false false))

(event `self.box.OnComponentBeginOverlap`
  (params (OverlappedComponent :type "PrimitiveComponent Object Reference") (OtherActor :type "Actor Object Reference") (OtherComp :type "PrimitiveComponent Object Reference") (OtherBodyIndex :type Integer) (bFromSweep :type Boolean) (SweepResult :type "HitResult Structure (by ref)"))
  (bind _asgliding_character (cast `/Game/FirstPersonBP/Blueprints/Gliding_Character` OtherActor))
  (bind _health (`/Game/FirstPersonBP/Blueprints/Gliding_Character.Health` _asgliding_character))
  (bind _maxhealth (`/Game/FirstPersonBP/Blueprints/Gliding_Character.MaxHealth` _asgliding_character))
  (if (< _health _maxhealth)
    (`KismetSystemLibrary.MoveComponentTo` (`self.Scene`) (`KismetMathLibrary.GetDirectionUnitVector` (`SceneComponent.K2_GetComponentLocation` (`self.Cube`)) (`SceneComponent.K2_GetComponentLocation` (`/Game/FirstPersonBP/Blueprints/Gliding_Character.FirstPersonCamera` _asgliding_character))) (struct) false false 0.3)
    (set `/Game/FirstPersonBP/Blueprints/Gliding_Character.Health` (`KismetMathLibrary.FClamp` (+ _health 20.0) 0.0 _maxhealth) _asgliding_character)
    (`KismetSystemLibrary.Delay` 0.1)
    (`self.K2_DestroyActor`)))

(fn `UserConstructionScript`)